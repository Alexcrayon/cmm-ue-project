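; BP_GAPAthComponent is a path component for AI characters whose Blueprint graph visualizes the current path for debugging.
; Each tick, when Debug is on and the path State is Active, it draws red lines between consecutive Steps points.
; A green line links the first step to the owning pawn's location.
; The graph only reads the path data and does no pathfinding or movement itself.
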(event `self.ReceiveTick`
  (params (DeltaSeconds :type "Float (single-precision)"))
  (if (`self.Debug`)
    (if (`|EnumEquality` (`self.State`) "GAPS_Active")
      (for (_ _array_index) (`self.Steps`)
        (if (> _array_index 0)
          (`KismetSystemLibrary.DrawDebugLine` (`.Point` (break `PathStep` (`|GetArrayItem` (`self.Steps`) _array_index))) (`.Point` (break `PathStep` (`|GetArrayItem` (`self.Steps`) (- _array_index 1)))) (struct :`R` 1.0 :`G` 0.034749 :`A` 1.0))))
      (if (`KismetArrayLibrary.Array_IsValidIndex` (`self.Steps`))
        (`KismetSystemLibrary.DrawDebugLine` (`.Point` (break `PathStep` (`|GetArrayItem` (`self.Steps`)))) (`Actor.K2_GetActorLocation` (`self.GetOwnerPawn`)) (struct :`G` 1.0 :`B` 0.097295 :`A` 1.0))))))