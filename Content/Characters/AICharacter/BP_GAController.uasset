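; BP_GAController is an AI character controller that makes its agent chase the first player's pawn.
; Every tick it feeds the player's current location to BPGACMMPathComponent as the path destination.
; BeginPlay turns on debug for GAPathComponent, although that component's SetDestination call is disconnected.
; A spatial component call that chooses and paths to a position is also left unwired.
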(event `self.ReceiveBeginPlay`
  (set `/Game/Characters/AICharacter/BP_GAPAthComponent.Debug` true (`self.GAPathComponent`)))

(event `self.ReceiveTick`
  (params (DeltaSeconds :type "Float (single-precision)"))
  (`GACMMPathComponent.SetDestination` (`self.BP_GACMMPathComponent`) (`self.K2_GetActorLocation` (`GameplayStatics.GetPlayerPawn` 0))))

(fn `UserConstructionScript`)